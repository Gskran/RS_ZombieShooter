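; Ammo pickup actor that refills a pawn's weapon of a matching type through focus and interact functions.
; Focus toggles custom depth on the mesh for the local player only, and an optional override material is applied at construction.
; Tooltip and pickupable checks depend on owning that weapon and having ammo below max.
; Pickup adds ammo and destroys the actor only on the server.
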(event EventSetFocused
  (params (InteractingPawn :type BP%20Player%20Character%20Object%20Reference) (IsFocused :type Boolean))
  (Rendering|SetRenderCustomDepth (Variables|Default|GetStaticMesh) (and (Pawn|IsLocallyControlled InteractingPawn) IsFocused)))

(fn ConstructionScript
  (bind _overridematerial (Variables|Default|GetOverrideMaterial))
  (Utilities|IsValid _overridematerial
    (:Is%20Valid
      (Rendering|Material|SetMaterial (Variables|Default|GetStaticMesh) 0 _overridematerial))))

(fn GetTooltipText
  (params (OwningPawn :type BP%20Player%20Character%20Object%20Reference))
  (bind _weapontype (Variables|Default|GetWeaponType))
  (bind (_hasweapon _theweapon) (Default|HasWeaponOfType OwningPawn _weapontype))
  (bind _displayname (Variables|/Game/GenericShooter/BlueprintLogic/Weapons/BP_BaseWeapon.BP_BaseWeapon_C|GetDisplayName _theweapon))
  (if _hasweapon
    (LocalVariables|SetOutText (select (< (Variables|/Game/GenericShooter/BlueprintLogic/Weapons/BP_BaseWeapon.BP_BaseWeapon_C|GetCurrentAmmo _theweapon) (Variables|/Game/GenericShooter/BlueprintLogic/Weapons/BP_BaseWeapon.BP_BaseWeapon_C|GetMaxAmmo _theweapon)) (Utilities|Text|FormatText "Press {Interact} To Pickup {WeaponName} Ammo" "E" _displayname) (Utilities|Text|FormatText "Already Have Max Ammo For {WeaponName}" _displayname)))
    (else
      (LocalVariables|SetOutText (Utilities|Text|FormatText "You Don't Have {WeaponName} For This Ammo" "A Suitable Weapon"))))
  (return (LocalVariables|GetOutText)))

(fn IsFocusable
  (params (OwningPawn :type BP%20Player%20Character%20Object%20Reference))
  (return true))

(fn IsPickupable
  (params (InteractingPawn :type BP%20Player%20Character%20Object%20Reference))
  (bind _weapontype (Variables|Default|GetWeaponType))
  (bind (_hasweapon _theweapon) (Default|HasWeaponOfType InteractingPawn _weapontype))
  (if _hasweapon
    (LocalVariables|SetOutCanPickup (< (Variables|/Game/GenericShooter/BlueprintLogic/Weapons/BP_BaseWeapon.BP_BaseWeapon_C|GetCurrentAmmo _theweapon) (Variables|/Game/GenericShooter/BlueprintLogic/Weapons/BP_BaseWeapon.BP_BaseWeapon_C|GetMaxAmmo _theweapon))))
  (return (LocalVariables|GetOutCanPickup)))

(fn Pickup
  (params (InteractingPawn :type BP%20Player%20Character%20Object%20Reference))
  (bind _weapontype (Variables|Default|GetWeaponType))
  (bind (_hasweapon _theweapon) (Default|HasWeaponOfType InteractingPawn _weapontype))
  (if _hasweapon
    (Networking|SwitchHasAuthority
      (:Authority
        (Default|AddAmmo _theweapon (Variables|Default|GetAmmoAmount) (Variables|Default|GetAddToClip) (Variables|Default|GetSkipMaxAmmoCheck))
        (Actor|DestroyActor))
      (:Remote
        _)))
  (return _hasweapon))